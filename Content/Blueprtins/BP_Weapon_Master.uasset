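; BP_Weapon_Master is a networked hitscan rifle, apparently a weapon base, with single and automatic fire, ammo and reload.
; The client sphere-traces from the camera with random spread, then from the muzzle to that point; automatic fire repeats this through a gated delay loop.
; The server trusts that hit to apply damage, decrements ammo, stops fire on empty and spawns impact and dual-mesh muzzle FX.
; Reload multicasts a sound, then refills the clip from reserve after a delay.
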(event `self.ReceiveBeginPlay`
  (`/Engine/EditorBlueprintResources/ActorMacros.Switch Has Authority`
    (:`Authority`
      (set `self.CurrentMaxAmmo` (`self.MaxAmmo`))
      (set `self.CurrentAmmoInClip` (`self.MaxAmmoClipSize`)))))

(event `Client_OnWeaponFire`
  (switch `/Game/Blueprtins/Enum/E_FiringMode` (`self.FiringMode`)
    (:`NewEnumerator0`
      _)
    (:`NewEnumerator1`
      (`self.AutoFireMode` :!label _label
        (:`then_0`
          _))))
  (bind (_outhit _hit _seeprojectilespawnloc _noseeprojectilespawnloc) (`self.SphereTrace`))
  (`self.Server_ShootInfo` _outhit _hit _seeprojectilespawnloc _noseeprojectilespawnloc))

(event `Server_ShootInfo`
  (params (OutHit :type "HitResult Structure (by ref)") (Hit :type Boolean) (SeeProjectileSpawnLoc :type "Vector Structure") (NoSeeProjectileSpawnLoc :type "Vector Structure"))
  (bind _currentammoinclip (`self.CurrentAmmoInClip`))
  (bind _bpmaincharacter (`self.BPMainCharacter`))
  (set `self.CurrentAmmoInClip` (`KismetMathLibrary.Clamp` (- _currentammoinclip 1) 0 (`self.CurrentMaxAmmo`)))
  (if (not (== _currentammoinclip 0))
    (`GameplayStatics.ApplyDamage` (`.HitActor` (`GameplayStatics.BreakHitResult` OutHit)) (`self.Base Damage`) (`self.GetInstigatorController`) self)
    (`self.StartFX` Hit OutHit)
    (else
      (`/Engine/EditorBlueprintResources/StandardMacros.IsValid` _bpmaincharacter
        (:`Is Valid`
          (`/Game/Blueprtins/BP_MainChracter.Server_StopWeaponFire` _bpmaincharacter))))))

(event `Client_OffWeaponFire`
  (`|ExecutionSequence`
    (:`then_0`
      (goto _label :!via `Close`))
    (:`then_1`
      (`self.StopFX`))))

(event `StartFX`
  (params (Hit :type Boolean) (`Out Hit` :type "HitResult Structure"))
  (`self.FireFX` Hit `Out Hit`)
  (switch `/Game/Blueprtins/Enum/E_FiringMode` (`self.FiringMode`)
    (:`NewEnumerator0`
      (`KismetSystemLibrary.Delay` 0.17)
      (`self.StopFX`))))

(event `StopFX`
  (bind _fpmuzzleflashref (`self.FPMuzzleFlashRef`))
  (`/Engine/EditorBlueprintResources/StandardMacros.IsValid` _fpmuzzleflashref
    (:`Is Valid`
      (`self.K2_DestroyActor` _fpmuzzleflashref))))

(event `Server_OnReloadWeapon`
  (`self.Multicast_ReloadFX`)
  (`KismetSystemLibrary.Delay` 2.0)
  (`self.ReloadAddAmmo`))

(event `Multicast_ReloadFX`
  (`GameplayStatics.SpawnSound2D` "/Game/MP_FPSBasic/Audio/Cues/A_Rifle_Reload_Cue.A_Rifle_Reload_Cue" 1.0 1.0 0.0 null))

(fn `FireFX`
  (params (Hit :type Boolean) (`Out Hit` :type "HitResult Structure"))
  (bind (_bblockinghit _binitialoverlap _time _distance _location _impactpoint _normal _impactnormal) (`GameplayStatics.BreakHitResult` `Out Hit`))
  (`|ExecutionSequence`
    (:`then_0`
      (`/Engine/EditorBlueprintResources/ActorMacros.Switch Has Authority`
        (:`Authority`
          (`/Engine/EditorBlueprintResources/StandardMacros.IsValid` (`self.FPMuzzleFlashRef`) ; 머즐 플래시가 없을때만 작동
            (:`Is Not Valid`
              (bind _returnvalue (`|SpawnActorFromClass` "/Game/Blueprtins/BP_FX_Fire.BP_FX_Fire_C" (`KismetMathLibrary.MakeTransform` (0.0 0.0 0.0)) "AdjustIfPossibleButAlwaysSpawn" "MultiplyWithRoot" (`self.GetOwner`) null))
              (bind _output_get (set `self.FPMuzzleFlashRef` _returnvalue))
              (`self.K2_AttachToActor` _output_get self "None" "KeepRelative" "KeepRelative" "KeepRelative" true)
              (`SceneComponent.K2_AttachToComponent` (`/Game/Blueprtins/BP_FX_Fire.MuzzleFlash_See` _output_get) (`self.SK_Rifle_See`) "Muzzle" "SnapToTarget" "SnapToTarget" "SnapToTarget" true)
              (`SceneComponent.K2_AttachToComponent` (`/Game/Blueprtins/BP_FX_Fire.MuzzleFlash_NoSee` _output_get) (`self.SK_Rifle_NoSee`) "Muzzle" "SnapToTarget" "SnapToTarget" "SnapToTarget" true))))))
    (:`then_1`
      (if Hit
        (`GameplayStatics.SpawnEmitterAtLocation` "/Game/MP_FPSBasic/Assets/MiscFX/Particles/PS_Rifle_Concrete_Impact.PS_Rifle_Concrete_Impact" _impactpoint (`KismetMathLibrary.MakeRotFromZ` _impactnormal))))))

(fn `ReloadAddAmmo`
  (locals (AmmoNeededforReload :type Integer))
  (`/Engine/EditorBlueprintResources/ActorMacros.Switch Has Authority`
    (:`Authority`
      (bind _output_get (set `local.AmmoNeededforReload` (- (`self.MaxAmmoClipSize`) (`self.CurrentAmmoInClip`))))
      (if (<= (`self.CurrentMaxAmmo`) _output_get)
        (set `self.CurrentAmmoInClip` (+ (`self.CurrentMaxAmmo`) (`self.CurrentAmmoInClip`)))
        (set `self.CurrentMaxAmmo` 0)
        (else
          (set `self.CurrentAmmoInClip` (`self.MaxAmmoClipSize`))
          (set `self.CurrentMaxAmmo` (- (`self.CurrentMaxAmmo`) (`local.AmmoNeededforReload`))))))))

(fn `SphereTrace`
  (returns (OutHit :type "HitResult Structure") (Hit :type Boolean) (SeeProjectileSpawnLoc :type "Vector Structure") (NoSeeProjectileSpawnLoc :type "Vector Structure"))
  (bind _returnvalue (`GameplayStatics.GetPlayerCameraManager` 0))
  (bind _returnvalue_2 (`PlayerCameraManager.GetCameraLocation` _returnvalue))
  (bind _returnvalue_3 (`SceneComponent.GetSocketLocation` (`self.SK_Rifle_See`) "Muzzle"))
  (bind _array (`|MakeArray` (`self.GetOwner`)))
  (bind (_outhit _returnvalue_4) (`KismetSystemLibrary.SphereTraceSingle` _returnvalue_2 (+ (+ _returnvalue_2 (* (`KismetMathLibrary.GetForwardVector` (`PlayerCameraManager.GetCameraRotation` _returnvalue)) 10000.0)) (* (`KismetMathLibrary.RandomFloatInRange` 0.0 300.0) (`KismetMathLibrary.RandomUnitVector`))) 2.0 "TraceTypeQuery1" false _array))
  (bind (_bblockinghit _binitialoverlap _time _distance _location _impactpoint _normal _impactnormal _physmat _hitactor _hitcomponent _hitbonename _bonename _hititem _elementindex _faceindex _tracestart _traceend) (`GameplayStatics.BreakHitResult` _outhit))
  (bind (_outhit_2 _returnvalue_5) (`KismetSystemLibrary.SphereTraceSingle` _returnvalue_3 (`KismetMathLibrary.SelectVector` _impactpoint _traceend _returnvalue_4) 2.0 "TraceTypeQuery1" false _array "ForDuration"))
  (return _outhit_2 _returnvalue_5 _returnvalue_3 (`SceneComponent.GetSocketLocation` (`self.SK_Rifle_NoSee`) "Muzzle")))

(fn `UserConstructionScript`)