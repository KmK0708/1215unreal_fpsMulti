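; BP_PC is a player controller that handles respawn requests and text chat for a multiplayer game.
; Server_Respawn asks BP_GM, the server-side game mode, to respawn this player.
; Enter focuses the chat widget's text box.
; Server_SendMessage prefixes the player name and relays the text to every BP_PC, whose client receive event updates that player's chat widget.
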(event `Server_Respawn`
  (bind _returnvalue (`GameplayStatics.GetGameMode`))
  (`/Engine/EditorBlueprintResources/StandardMacros.IsValid` _returnvalue
    (:`Is Valid`
      (bind _asbp_gm (cast `/Game/Blueprtins/GameMode/BP_GM` _returnvalue))
      (`/Game/Blueprtins/GameMode/BP_GM.Server_RespawnPlayer` _asbp_gm self))))

(event `Key|Enter`
  (params (Key :type "Key Structure"))
  (bind _editabletextbox_105 (`/Game/UI/WB_Chatting.EditableTextBox_105` (`self.WB_Chatting`)))
  ;[1 1 1] 엔터 누르면 채팅 ui에 에디터블 박스에 포커스
  (:`Pressed`
    (if (not (`Widget.HasKeyboardFocus` _editabletextbox_105))
      (`Widget.SetFocus` _editabletextbox_105))))

(event `Server_SendMessage`
  (params (`In Text` :type Text))
  ;[1 1 1] 메세지를 서버에서 보낸다
  (bind _outactors (`GameplayStatics.GetAllActorsOfClass` "BP_PC_C"))
  (for _array_element _outactors
    (`self.Client_ReceiveMessage` _array_element (`KismetTextLibrary.Conv_StringToText` (`KismetStringLibrary.Concat_StrStr` (`PlayerState.GetPlayerName` (`self.PlayerState`)) ":" (`KismetTextLibrary.Conv_TextToString` `In Text`))))))

(event `Client_ReceiveMessage`
  (params (`In Text` :type Text))
  (bind _wb_chatting (`self.WB_Chatting`))
  ;[1 1 1] 받는거는 각자가 받는거니 클라이언트
  (`/Engine/EditorBlueprintResources/StandardMacros.IsValid` _wb_chatting
    (:`Is Valid`
      (`/Game/UI/WB_Chatting.UpdateChat` _wb_chatting `In Text`))))

(fn `UserConstructionScript`)