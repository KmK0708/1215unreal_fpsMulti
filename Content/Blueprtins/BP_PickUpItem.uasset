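; BP_PickUpItem is a respawning ammo pickup that BP_MainChracter collects by overlapping it.
; On authority, the overlap calls Server_OnExplosivePickup, which adds AmountToGive to the current weapon's CurrentMaxAmmo, clamped between zero and MaxAmmo.
; It then sets IsHidden for RespawnTime before clearing it.
; The IsHidden RepNotify toggles actor visibility and sphere collision, so the same actor is reused rather than destroyed.
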(event `self.ReceiveActorBeginOverlap`
  (params (OtherActor :type "Actor Object Reference"))
  (`/Engine/EditorBlueprintResources/ActorMacros.Switch Has Authority`
    (:`Authority`
      (bind _asbp_main_chracter (cast `/Game/Blueprtins/BP_MainChracter` OtherActor))
      (`self.Server_OnExplosivePickup` _asbp_main_chracter)
      (set `self.IsHidden?` true)
      (`KismetSystemLibrary.Delay` (`self.RespawnTime`))
      (set `self.IsHidden?` false))))

(event `Server_OnExplosivePickup`
  (params (MainCharacter :type "/Game/Blueprtins/BP_MainChracter Object Reference"))
  (bind _currentweapon (`/Game/Blueprtins/BP_MainChracter.CurrentWeapon` MainCharacter))
  (set `/Game/Blueprtins/BP_Weapon_Master.CurrentMaxAmmo` (`KismetMathLibrary.Clamp` (+ (`/Game/Blueprtins/BP_Weapon_Master.CurrentMaxAmmo` _currentweapon) (`self.AmountToGive`)) 0 (`/Game/Blueprtins/BP_Weapon_Master.MaxAmmo` _currentweapon)) _currentweapon))

(fn `OnRep_IsHidden?`
  (if (`self.IsHidden?`)
    (`PrimitiveComponent.SetCollisionEnabled` (`self.Sphere`) "NoCollision")
    (`self.SetActorHiddenInGame` true)
    (else
      (`PrimitiveComponent.SetCollisionEnabled` (`self.Sphere`) "QueryAndPhysics")
      (`self.SetActorHiddenInGame` false))))

(fn `UserConstructionScript`)